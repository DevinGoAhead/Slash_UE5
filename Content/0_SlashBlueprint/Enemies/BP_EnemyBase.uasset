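; Base enemy Blueprint that keeps motion-warping targets aligned with its combat target.
; On Tick, while CombatTarget is valid, it feeds computed translation and rotation locations into the MotionWarping component as named warp targets.
; Disconnected leftover nodes for pawn sensing, which would chase a seen BP_SlashCharacter at a set walk speed, never run.
; BeginPlay and the construction script are empty.
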(event Custom|OnSeePawn_Event
  (params (Pawn :type Pawn%20Object%20Reference)))

(event EventBeginPlay)

(event Collision|EventActorBeginOverlap
  (params (OtherActor :type Actor%20Object%20Reference)))

(event EventTick
  (params (DeltaSeconds :type Float%20%28single-precision%29))
  (Variables|Default|GetCombatTarget
    (:then
      (bind _returnvalue (Class|Enemy|GetTranslationWarpTarget))
      (Class|MotionWarpingComponent|AddorUpdateWarpTargetfromLocation (Variables|Default|GetMotionWarping) "TranslationTarget" _returnvalue)
      (bind _returnvalue_2 (Class|Enemy|GetRotationWarpTarget))
      (Class|MotionWarpingComponent|AddorUpdateWarpTargetfromLocation (Variables|Default|GetMotionWarping) "RotationTarget" _returnvalue_2))
    (:else)))

(fn ConstructionScript)